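; BP_Mage is the player-controlled Mage character Blueprint, handling third- or first-person style movement, camera look and sprinting.
; Movement axes add input along forward and right vectors built from control rotation yaw only, so pitch does not affect direction.
; Camera axes feed controller pitch and yaw input.
; The Sprint action sets a SprintPressed flag and switches CharacterMovement max walk speed between running and normal values.
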(event Input|ActionEvents|InputActionSprint
  (params (Key :type Key%20Structure :default "AnyKey"))
  (bind _charactermovement (Variables|Character|GetCharacterMovement))
  ;[1 1 1] Sprint Input
  (:Pressed
    (Variables|Default|SetSprintPressed true)
    (Variables|/Script/Engine.CharacterMovementComponent|SetMaxWalkSpeed _charactermovement 1e+03))
  (:Released
    (Variables|Default|SetSprintPressed false)
    (Variables|/Script/Engine.CharacterMovementComponent|SetMaxWalkSpeed _charactermovement 6e+02)))

(event Input|AxisEvents|InputAxisMoveForward/Backward
  (params (AxisValue :type Float%20%28single-precision%29))
  ;[1 1 1] Input for Character Movement
  (Pawn|Input|AddMovementInput (Math|Vector|GetForwardVector (Math|Rotator|MakeRotator 0.0 0.0 (.Yaw (Math|Rotator|BreakRotator (Pawn|GetControlRotation :!class /Script/Engine.Pawn))))) AxisValue false))

(event Input|AxisEvents|InputAxisMoveRight/Left
  (params (AxisValue :type Float%20%28single-precision%29))
  ;[1 1 1] Input for Character Movement
  (Pawn|Input|AddMovementInput (Math|Vector|GetRightVector (Math|Rotator|MakeRotator 0.0 0.0 (.Yaw (Math|Rotator|BreakRotator (Pawn|GetControlRotation :!class /Script/Engine.Pawn))))) AxisValue false))

(event Input|AxisEvents|InputAxisCameraUp/Down
  (params (AxisValue :type Float%20%28single-precision%29))
  ;[1 1 1] Input For Camera Movement
  (Pawn|Input|AddControllerPitchInput AxisValue))

(event Input|AxisEvents|InputAxisCameraRight/Left
  (params (AxisValue :type Float%20%28single-precision%29))
  ;[1 1 1] Input For Camera Movement
  (Pawn|Input|AddControllerYawInput AxisValue))

(fn ConstructionScript)