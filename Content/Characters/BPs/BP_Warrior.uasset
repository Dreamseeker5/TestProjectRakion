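; BP_Warrior is a character Blueprint that handles input for movement, camera, sprinting, sideways evades and blocking.
; Movement follows control yaw, sprint raises walk speed, and DisableMovement suspends normal movement during block or evade.
; Evades set timed flags that the Move Right/Left axis event turns into forced sideways input until a delay clears them.
; A forward evade sequence exists but is not connected to any event.
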(event Input|ActionEvents|InputActionSprint
  (params (Key :type Key%20Structure :default "AnyKey"))
  (bind _charactermovement (Variables|Character|GetCharacterMovement))
  ;[1 1 1] Sprint Input
  (:Pressed
    (Variables|Default|SetSprint%20Pressed true)
    (Variables|/Script/Engine.CharacterMovementComponent|SetMaxWalkSpeed _charactermovement 1e+03))
  (:Released
    (Variables|Default|SetSprint%20Pressed false)
    (Variables|/Script/Engine.CharacterMovementComponent|SetMaxWalkSpeed _charactermovement 6e+02)))

(event Input|ActionEvents|InputActionEvade/Front
  (params (Key :type Key%20Structure :default "AnyKey"))
  ;[1 1 1] Evading Input
)

(event Input|ActionEvents|InputActionEvade/Left
  (params (Key :type Key%20Structure :default "AnyKey"))
  ;[1 1 1] Evading Input
  (:Pressed
    (Variables|Default|SetEvade%20LPressed true)
    (Variables|Default|SetDisable%20Movement true)
    (Utilities|FlowControl|Delay 0.6)
    (Variables|Default|SetEvade%20LPressed false)
    (Variables|Default|SetDisable%20Movement false)))

(event Input|ActionEvents|InputActionBlock
  (params (Key :type Key%20Structure :default "AnyKey"))
  ;[1 1 1] Block input
  (:Pressed
    (Variables|Default|SetBlock%20Pressed true)
    (Variables|Default|SetDisable%20Movement true))
  (:Released
    (Variables|Default|SetBlock%20Pressed false)
    (Variables|Default|SetDisable%20Movement false)))

(event Input|ActionEvents|InputActionEvade/Right
  (params (Key :type Key%20Structure :default "AnyKey"))
  ;[1 1 1] Evading Input
  (:Pressed
    (Variables|Default|SetEvade%20RPressed true)
    (Variables|Default|SetDisable%20Movement true)
    (Utilities|FlowControl|Delay 0.6)
    (Variables|Default|SetEvade%20RPressed false)
    (Variables|Default|SetDisable%20Movement false)))

(event Input|AxisEvents|InputAxisMoveForward/Backward
  (params (AxisValue :type Float%20%28single-precision%29))
  ;[1 1 1] Input for Character Movement
  (if (not (Variables|Default|GetDisable%20Movement))
    (Pawn|Input|AddMovementInput (Math|Vector|GetForwardVector (Math|Rotator|MakeRotator 0.0 0.0 (.Yaw (Math|Rotator|BreakRotator (Pawn|GetControlRotation :!class /Script/Engine.Pawn))))) AxisValue false)))

(event Input|AxisEvents|InputAxisMoveRight/Left
  (params (AxisValue :type Float%20%28single-precision%29))
  (bind _returnvalue (Pawn|GetControlRotation :!class /Script/Engine.Pawn))
  (bind _evade_rpressed (Variables|Default|GetEvade%20RPressed))
  (bind _yaw (Math|Rotator|BreakRotator _returnvalue))
  (bind _returnvalue_2 (Math|Rotator|MakeRotator 0.0 0.0 _yaw))
  (bind _returnvalue_3 (Math|Vector|GetRightVector _returnvalue_2))
  ;[1 1 1] Input for Character Movement
  (if (Variables|Default|GetDisable%20Movement)
    (if (or _evade_rpressed (Variables|Default|GetEvade%20LPressed))
      (if _evade_rpressed
        (Pawn|Input|AddMovementInput _returnvalue_3 2.0 false)
        (else
          (Pawn|Input|AddMovementInput _returnvalue_3 -2.0 false))))
    (else
      (Pawn|Input|AddMovementInput _returnvalue_3 AxisValue false))))

(event Input|AxisEvents|InputAxisCameraUp/Down
  (params (AxisValue :type Float%20%28single-precision%29))
  ;[1 1 1] Input For Camera Movement
  (Pawn|Input|AddControllerPitchInput AxisValue))

(event Input|AxisEvents|InputAxisCameraRight/Left
  (params (AxisValue :type Float%20%28single-precision%29))
  ;[1 1 1] Input For Camera Movement
  (Pawn|Input|AddControllerYawInput AxisValue))

(fn ConstructionScript)